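; BP_BallSpawner is a chute actor that spawns BP_Ball projectiles in the chute's color.
; SetChuteColor creates a dynamic material instance on ChuteMesh and writes its Color parameter.
; SpawnBall spawns a ball at the actor's location, copies that Color to it and sets its projectile InitialSpeed after spawning.
; Color and speed are applied only if the chute material is already a dynamic instance.
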(event Custom|SpawnBall
  (bind _returnvalue (Game|SpawnActorfromClass "/Game/Blueprints/BP_Ball.BP_Ball_C" (Math|Transform|MakeTransform (Transformation|GetActorLocation)) "Undefined" 0 0))
  (bind _asmaterial_instance_dynamic (Utilities|Casting|CastToMaterialInstanceDynamic (Rendering|Material|GetMaterial (Variables|Default|GetChuteMesh) 0)))
  (bind _returnvalue_2 (Rendering|Material|GetVectorParameterValue _asmaterial_instance_dynamic "Color" :!class /Script/Engine.MaterialInstanceDynamic))
  (Default|SetColor _returnvalue _returnvalue_2)
  (Variables|/Script/Engine.ProjectileMovementComponent|SetInitialSpeed (Variables|/Game/Blueprints/BP_Ball.BP_Ball_C|GetProjectile _returnvalue) 2e+03))

(event EventBeginPlay)

(event Collision|EventActorBeginOverlap
  (params (OtherActor :type Actor%20Object%20Reference)))

(event EventTick
  (params (DeltaSeconds :type Float%20%28single-precision%29)))

(fn ConstructionScript)

(fn SetChuteColor
  (params (Color :type Linear%20Color%20Structure))
  (bind _returnvalue (Rendering|Material|CreateDynamicMaterialInstance (Variables|Default|GetChuteMesh) 0 0 "None" :!class /Script/Engine.PrimitiveComponent))
  (Rendering|Material|SetVectorParameterValue _returnvalue "Color" Color :!class /Script/Engine.MaterialInstanceDynamic))