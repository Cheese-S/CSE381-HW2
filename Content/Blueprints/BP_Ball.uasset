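; BP_Ball is a colored ball pickup that reloads an FPSchar that has no ammo.
; On overlap, it grants ammo, plays a reload sound, copies its material's Color to the character and destroys itself.
; A Leftspawn flag ignores overlaps for a short delay after spawn.
; SetColor applies a given color through a dynamic material instance, while EventSetColor applies a fixed green.
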(event Custom|EventSetColor
  (bind _returnvalue (Rendering|Material|CreateDynamicMaterialInstance (Variables|Default|GetBallMesh) 0 0 "None" :!class /Script/Engine.PrimitiveComponent))
  (Rendering|Material|SetVectorParameterValue _returnvalue "Color" "(R=0.149960,G=0.896269,B=0.149960,A=1.000000)" :!class /Script/Engine.MaterialInstanceDynamic))

(event EventBeginPlay
  (Variables|Default|Setleftspawn false)
  (Utilities|FlowControl|Delay 0.2)
  (Variables|Default|Setleftspawn true))

(event Collision|EventActorBeginOverlap
  (params (OtherActor :type Actor%20Object%20Reference))
  (if (Variables|Default|Getleftspawn)
    (bind _asfpschar (Utilities|Casting|CastToFPSchar OtherActor))
    (if (not (Variables|/Game/BP/FPSchar.FPSchar_C|Gethas_ammo _asfpschar))
      (Variables|/Game/BP/FPSchar.FPSchar_C|Sethas_ammo _asfpschar true)
      (Utilities|FlowControl|Sequence
        (:then_0
          (Audio|SpawnSoundatLocation "/Game/MilitaryWeapDark/Sound/GrenadeLauncher/Wavs/GrenadeLauncher_ReloadInsert01.GrenadeLauncher_ReloadInsert01" (Transformation|GetActorLocation) "0, 0, 0" 1.0 1.0 0.0 0 0))
        (:then_1
          (bind _asmaterial_instance_dynamic (Utilities|Casting|CastToMaterialInstanceDynamic (Rendering|Material|GetMaterial (Variables|Default|GetBallMesh) 0)))
          (bind _returnvalue (Rendering|Material|GetVectorParameterValue _asmaterial_instance_dynamic "Color" :!class /Script/Engine.MaterialInstanceDynamic))
          (Variables|/Game/BP/FPSchar.FPSchar_C|SetColor _asfpschar _returnvalue))
        (:then_2
          (Actor|DestroyActor))))))

(event EventTick
  (params (DeltaSeconds :type Float%20%28single-precision%29)))

(fn ConstructionScript)

(fn SetColor
  (params (Color :type Linear%20Color%20Structure))
  (bind _returnvalue (Rendering|Material|CreateDynamicMaterialInstance (Variables|Default|GetBallMesh) 0 0 "None" :!class /Script/Engine.PrimitiveComponent))
  (Rendering|Material|SetVectorParameterValue _returnvalue "Color" Color :!class /Script/Engine.MaterialInstanceDynamic))