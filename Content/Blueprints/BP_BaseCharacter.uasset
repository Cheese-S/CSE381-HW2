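; Base first-person character that picks up colored BP_Balls and fires balls of the stored color.
; Overlapping a ball with Leftspawn set while empty stores its color, destroys it and sets HasAmmo, which shows a tinted held-ball mesh via a dynamic material.
; Fire spawns a ball at that mesh along camera rotation, once per press via DoOnce, whether or not HasAmmo is set, and never clears that flag.
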(event EventBeginPlay)

(event Collision|EventActorBeginOverlap
  (params (OtherActor :type Actor%20Object%20Reference))
  (bind _holdballmesh (Variables|Default|GetHoldBallMesh))
  (Utilities|FlowControl|Sequence
    (:then_0
      (bind _asbp_ball (Utilities|Casting|CastToBP_Ball OtherActor))
      (if (Variables|/Game/Blueprints/BP_Ball.BP_Ball_C|Getleftspawn _asbp_ball)
        (if (not (Variables|Default|GetHasAmmo))
          (Variables|Default|SetHasAmmo true)
          (bind _color (Default|GetColor _asbp_ball))
          (Variables|Default|SetColor _color)
          (Actor|DestroyActor OtherActor))))
    (:then_1
      (if (Variables|Default|GetHasAmmo)
        (Rendering|SetVisibility _holdballmesh true false)
        (bind _returnvalue (Rendering|Material|CreateDynamicMaterialInstance _holdballmesh 0 0 "None" :!class /Script/Engine.PrimitiveComponent))
        (Rendering|Material|SetVectorParameterValue _returnvalue "Color" (Variables|Default|GetColor) :!class /Script/Engine.MaterialInstanceDynamic)
        (else
          (Rendering|SetVisibility _holdballmesh false false))))))

(event EventTick
  (params (DeltaSeconds :type Float%20%28single-precision%29)))

(event Input|ActionEvents|InputActionFire
  (params (Key :type Key%20Structure :default "None"))
  (:Pressed
    (Utilities|FlowControl|DoOnce false :!label _label
      (:Completed
        (if (Variables|Default|GetHasAmmo)
          (Variables|Default|SetHasAmmo true))
        (bind _returnvalue (Game|SpawnActorfromClass "/Game/Blueprints/BP_Ball.BP_Ball_C" (Math|Transform|MakeTransform (Transformation|GetSocketLocation (Variables|Default|GetHoldBallMesh) "None") (Transformation|GetWorldRotation (Variables|Default|GetFPSCameraComponent)) "0.700000,0.700000,0.700000") "Undefined" 0 0))
        (Default|SetColor _returnvalue (Variables|Default|GetColor)))))
  (:Released
    (goto _label Reset)))

(fn ConstructionScript)