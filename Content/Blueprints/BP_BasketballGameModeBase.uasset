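; Game mode for a basketball game that tracks the score and handles game over and restart.
; It shows the game widget on BeginPlay; baskets score only when their color alternates between blue and orange, tracked by a toggled boolean.
; Game over shows its widget, switches to UI input with a cursor, saves the high score to the game instance and pauses.
; Restart hides the cursor and restores game-only input.
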(event Custom|OnGameRestart
  (bind _returnvalue (Game|GetPlayerController 0))
  (Variables|/Script/Engine.PlayerController|SetbShowMouseCursor _returnvalue false)
  (Input|SetInputModeGameOnly _returnvalue))

(event Custom|OnGameOver
  (bind _returnvalue (Game|GetPlayerController 0))
  (bind _returnvalue_2 (UserInterface|CreateWidget "/Game/Blueprints/GameOverWidget.GameOverWidget_C" _returnvalue))
  (UserInterface|Viewport|AddtoViewport _returnvalue_2 0)
  (Input|SetInputModeUIOnly _returnvalue 0 "DoNotLock")
  (Variables|/Script/Engine.PlayerController|SetbShowMouseCursor (Game|GetPlayerController 0) true)
  (bind _asbp_game_instance (Utilities|Casting|CastToBP_GameInstance (Game|GetGameInstance)))
  (Variables|/Game/Blueprints/BP_GameInstance.BP_GameInstance_C|SetHighScore _asbp_game_instance (Math|Integer|Max(Integer) (Variables|Default|GetCurrentScore) (Variables|/Game/Blueprints/BP_GameInstance.BP_GameInstance_C|GetHighScore _asbp_game_instance)))
  (Game|SetGamePaused true))

(event Custom|OnBasketMade
  (params (Color :type Linear%20Color%20Structure))
  (if (Variables|Default|GetWhichColor)
    (if (== Color (Variables|Default|GetBlue))
      (Math|Integer|IncrementInt (Variables|Default|GetCurrentScore) :!label _label
        (:%20%20
          (Variables|Default|SetWhichColor (not (Variables|Default|GetWhichColor))))))
    (elif (== Color (Variables|Default|GetOrange))
      (goto _label))))

(event EventBeginPlay
  (bind _returnvalue (UserInterface|CreateWidget "/Game/Blueprints/GameWidget.GameWidget_C" (Game|GetPlayerController 0)))
  (UserInterface|Viewport|AddtoViewport _returnvalue 0))

(event EventTick
  (params (DeltaSeconds :type Float%20%28single-precision%29)))

(fn ConstructionScript)