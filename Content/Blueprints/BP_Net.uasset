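; BP_Net is a basketball net that scores a basket when a ball of the same color enters it.
; On CollisionMesh overlap, it compares the BP_Ball's color with its own, destroys a matching ball and notifies BP_BasketballGameModeBase through OnBasketMade.
; The net's color lives in the "Color" material parameter on NetMesh, with both setter and getter calling CreateDynamicMaterialInstance on each use.
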(event OnComponentBeginOverlap(CollisionMesh)
  (params (OverlappedComponent :type Primitive%20Component%20Object%20Reference) (OtherActor :type Actor%20Object%20Reference) (OtherComp :type Primitive%20Component%20Object%20Reference) (OtherBodyIndex :type Integer) (bFromSweep :type Boolean) (SweepResult :type Hit%20Result%20Structure%20%28by%20ref%29))
  (bind _asbp_ball (Utilities|Casting|CastToBP_Ball OtherActor))
  (bind _color (Default|GetColor _asbp_ball))
  (bind _color_2 (CallFunction|GetNetColor))
  (if (== _color _color_2)
    (Actor|DestroyActor OtherActor)
    (bind _asbp_basketball_game_mode_base (Utilities|Casting|CastToBP_BasketballGameModeBase (Game|GetGameMode)))
    (Default|OnBasketMade _asbp_basketball_game_mode_base _color_2)))

(event EventBeginPlay)

(event Collision|EventActorBeginOverlap
  (params (OtherActor :type Actor%20Object%20Reference)))

(event EventTick
  (params (DeltaSeconds :type Float%20%28single-precision%29)))

(fn ConstructionScript)

(fn SetNetColor
  (params (Color :type Linear%20Color%20Structure))
  (bind _returnvalue (Rendering|Material|CreateDynamicMaterialInstance (Variables|Default|GetNetMesh) 0 0 "None" :!class /Script/Engine.PrimitiveComponent))
  (Rendering|Material|SetVectorParameterValue _returnvalue "Color" Color :!class /Script/Engine.MaterialInstanceDynamic))

(fn GetNetColor
  (bind _returnvalue (Rendering|Material|CreateDynamicMaterialInstance (Variables|Default|GetNetMesh) 0 0 "Color" :!class /Script/Engine.PrimitiveComponent))
  (bind _returnvalue_2 (Rendering|Material|GetVectorParameterValue _returnvalue "Color" :!class /Script/Engine.MaterialInstanceDynamic))
  (return _returnvalue_2))